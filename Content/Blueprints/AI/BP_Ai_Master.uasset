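; Master AI character Blueprint that handles health, a socket-attached weapon, damage reactions and ragdoll death.
; Hits play a random montage and feed bone-based damage with a headshot multiplier, spawning floating text and counting headshots.
; A looping timer polls for death, while radial damage checks immediately as a grenade kill.
; Death drops the weapon actor via destruction and credits player kill counters, with delayed self-destruction only for non-grenade kills.
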(event Custom|CheckDeath
  ;[1 1 1] Beginning
  (CallFunction|Death false))

(event Custom|EventDestroy
  (params (Delay :type Float%20%28single-precision%29) (Target :type Actor%20Object%20Reference))
  ;[1 1 1] Destroy Actor
  (Utilities|DestroyMacro Delay Target))

(event Game|Damage|EventRadialDamage
  (params (DamageReceived :type Float%20%28single-precision%29) (DamageType :type Damage%20Type%20Object%20Reference) (Origin :type Vector :default "0, 0, 0") (HitInfo :type Hit%20Result%20Structure%20%28by%20ref%29) (InstigatedBy :type Controller%20Object%20Reference) (DamageCauser :type Actor%20Object%20Reference))
  ;[1 1 1] Taking damage
  (CallFunction|CalculateDamage "None" DamageReceived)
  (CallFunction|Death true))

(event EventBeginPlay
  ;[1 1 1] Beginning
  (CallFunction|SetHealth)
  (CallFunction|SnapWeapon)
  (bind _returnvalue (Utilities|Time|SetTimerbyEvent (delegate Custom|CheckDeath) 0.1 true))
  (Variables|Default|SetTimer _returnvalue)
  (bind _asbp_player_character (Utilities|Casting|CastToBP_PlayerCharacter (Game|GetPlayerCharacter 0)))
  (Variables|Default|SetPlayerCharacterRef _asbp_player_character))

(event EventTakingDamage
  (params (Bone :type Name :default "None") (Damage :type Float%20%28single-precision%29) (Instigator :type Actor%20Object%20Reference))
  ;[1 1 1] Taking damage
  (Animation|Montage|PlayMontage (Variables|Character|GetMesh) (Utilities|Array|Get(acopy) (Variables|Default|GetHitReactArray) (Math|Random|RandomIntegerinRange 0 3))
    (:then
      (CallFunction|CalculateDamage Bone Damage Instigator))))

(fn ConstructionScript)

(fn SetHealth
  (Variables|Default|SetCurrentHealth (Variables|Default|GetMaxHealth)))

(fn Death
  (params (IsGrenade :type Boolean))
  (bind _mesh (Variables|Character|GetMesh))
  (bind _playercharacterref (Variables|Default|GetPlayerCharacterRef))
  (if (<= (Variables|Default|GetCurrentHealth) 0.0)
    (Class|SkeletalMeshComponent|SetAllBodiesSimulatePhysics _mesh true)
    (Collision|SetCollisionProfileName _mesh "Ragdoll" true :!class /Script/Engine.PrimitiveComponent)
    (Collision|SetCollisionEnabled (Variables|Collision|GetCapsuleComponent) "NoCollision")
    (Actor|DestroyActor (Variables|Default|GetWeaponActor))
    (Utilities|Time|PauseTimerbyHandle (Variables|Default|GetTimer))
    (if IsGrenade
      (Default|IncreaseCounter _playercharacterref "HandGrenade")
      (else
        (Default|IncreaseCounter _playercharacterref (Variables|/Game/Blueprints/Weapon/BP_Weapon_Master.BP_Weapon_Master_C|GetWeaponType (Variables|/Game/Blueprints/Player/BP_PlayerCharacter.BP_PlayerCharacter_C|GetWeaponMasterRef _playercharacterref)))
        (CallFunction|EventDestroy (LocalVariables|GetTimeDelay) self)))))

(fn CalculateDamage
  (params (Bone :type Name) (Damage :type Float%20%28single-precision%29) (Instigator :type Actor%20Object%20Reference))
  (bind _returnvalue (== Bone "head"))
  (bind _mesh (Variables|Character|GetMesh))
  (bind _returnvalue_2 (Physics|IsSimulatingPhysics _mesh "None"))
  (bind _returnvalue_3 (not _returnvalue_2))
  (LocalVariables|SetDamageLoc Damage)
  (if _returnvalue
    (Variables|Default|SetCurrentHealth (- (Variables|Default|GetCurrentHealth) (* (LocalVariables|GetDamageLoc) (LocalVariables|GetDamageMultiplier))))
    (bind _asbp_player_character (Utilities|Casting|CastToBP_PlayerCharacter Instigator))
    (if _returnvalue_3
      (Default|IncreaseCounter _asbp_player_character "Headshot")
      (Game|SpawnActorfromClass "/Game/Blueprints/Weapon/DamageText/BP_FloatingText.BP_FloatingText_C" (Math|Transform|MakeTransform (Transformation|GetActorLocation) "0, 0, 0" "1,1,1") "Undefined" 0 (select _returnvalue "Headshot" (Utilities|Text|ToText(Float) (LocalVariables|GetDamageLoc) "HalfToEven" false true 1 324 0 0)) 0 :!label _label))
    (else
      (Variables|Default|SetCurrentHealth (- (Variables|Default|GetCurrentHealth) (LocalVariables|GetDamageLoc)))
      (if _returnvalue_3
        (goto _label)))))

(fn SnapWeapon
  (bind _mesh (Variables|Character|GetMesh))
  (bind _returnvalue (Game|SpawnActorfromClass (Variables|Default|GetWeaponClass) (Transformation|GetSocketTransform _mesh "skt_gun1" "RTS_ParentBoneSpace") "Undefined" 0 0))
  (bind _output_get (Variables|Default|SetWeaponActor _returnvalue))
  (Transformation|AttachComponentToComponent _output_get (Variables|Character|GetMesh) (Class|SkinnedMeshComponent|GetSocketBoneName _mesh "skt_gun1") "KeepRelative" "KeepRelative" "KeepRelative" true))