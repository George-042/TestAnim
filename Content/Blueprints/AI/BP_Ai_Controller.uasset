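; AI controller that switches its pawn between patrolling and attacking behavior trees.
; It starts on the patrol tree, and when PawnSensing sees a pawn it runs the attack tree and writes that pawn to a blackboard key.
; A ten-second timer then fires TargetLost to return to patrol.
; SetTargetActor also writes a given actor to the blackboard.
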(event OnSeePawn(PawnSensing)
  (params (Pawn :type Pawn%20Object%20Reference))
  (AI|RunBehaviorTree "/Game/Blueprints/AI/BT_AiAttack.BT_AiAttack")
  (AI|Components|Blackboard|SetValueasObject (Variables|Default|GetBlackboard) (Variables|Default|GetKeyName) Pawn)
  (Utilities|Time|SetTimerbyEvent (delegate Custom|TargetLost) 1e+01))

(event Custom|TargetLost
  (AI|RunBehaviorTree "/Game/Blueprints/AI/BT_AiPatrol.BT_AiPatrol"))

(event EventBeginPlay
  (AI|RunBehaviorTree "/Game/Blueprints/AI/BT_AiPatrol.BT_AiPatrol"))

(fn ConstructionScript)

(fn SetTargetActor
  (params (TargetActor :type Actor%20Object%20Reference))
  (AI|Components|Blackboard|SetValueasObject (Variables|Default|GetBlackboard) (Variables|Default|GetKeyName) TargetActor))