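; BP_FloatingText is a short-lived actor that shows floating damage text rising from where it spawns.
; On BeginPlay it creates a WD_FloatingText widget from its DamageText value, assigns it to its Widget component and sets a one-second lifespan.
; Each Tick nudges that component upward in relative space by a random step, not scaled by delta time, so the rise is uneven and frame-rate dependent.
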(event EventBeginPlay
  (bind _returnvalue (UserInterface|CreateWidget "/Game/UMG/GameLevel/WD_FloatingText.WD_FloatingText_C" 0 (Variables|Default|GetDamageText)))
  (UserInterface|SetWidget (Variables|Default|GetWidget) _returnvalue)
  (Actor|SetLifeSpan 1.0))

(event EventTick
  (params (DeltaSeconds :type Float%20%28single-precision%29))
  (bind _widget (Variables|Default|GetWidget))
  (Transformation|SetRelativeLocation _widget (+ (Variables|/Script/Engine.SceneComponent|GetRelativeLocation _widget) (Math|Vector|MakeVector 0.0 0.0 (Math|Random|RandomFloatinRange 0.5 2.0))) false false))

(fn ConstructionScript)