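; Master projectile actor that resolves hits as either a bullet or a rocket, based on its Type.
; BeginPlay copies Speed into the projectile movement's initial speed.
; Bullets send bone-specific damage through BPI_TakeDamage, or otherwise push physics objects and leave stone impact effects and temporary attached hole decals.
; Rockets spawn an explosion with sound and apply radial damage; both types destroy themselves on hit.
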(event EventBeginPlay
  (Variables|/Script/Engine.ProjectileMovementComponent|SetInitialSpeed (Variables|Default|GetProjectileMovement) (Variables|Default|GetSpeed)))

(event Collision|EventHit
  (params (MyComp :type Primitive%20Component%20Object%20Reference) (Other :type Actor%20Object%20Reference) (OtherComp :type Primitive%20Component%20Object%20Reference) (bSelfMoved :type Boolean) (HitLocation :type Vector :default "0, 0, 0") (HitNormal :type Vector :default "0, 0, 0") (NormalImpulse :type Vector :default "0, 0, 0") (Hit :type Hit%20Result%20Structure%20%28by%20ref%29))
  (bind _returnvalue (Physics|IsSimulatingPhysics OtherComp "None"))
  (bind (_bblockinghit _binitialoverlap _time _distance _location _impactpoint _normal _impactnormal _physmat _hitactor _hitcomponent _hitbonename) (Collision|BreakHitResult Hit))
  (bind _returnvalue_2 (Transformation|GetWorldTransform OtherComp))
  (switch Utilities|FlowControl|Switch|SwitchonEnum_ProjectileType (Variables|Default|GetType)
    (:NewEnumerator0
      (if (Utilities|DoesObjectImplementInterface Other "/Game/Blueprints/Player/BPI_TakeDamage.BPI_TakeDamage_C")
        (Class|BPITakeDamage|TakingDamage(Message) _hitactor _hitbonename (Variables|Default|GetDamage) (Game|GetInstigator))
        (if _returnvalue
          _
          (else
            _))
        (else
          (if _returnvalue
            (Physics|AddImpulseatLocation OtherComp (* (Transformation|GetVelocity) 1e+01) (Transformation|GetActorLocation) "None"))
          (Effects|SpawnEmitteratLocation "/Game/Assets/FX/P_Impact_Stone_Medium_01.P_Impact_Stone_Medium_01" _impactpoint)
          (bind _returnvalue_3 (Class|GameplayStatics|SpawnDecalAttached "/Game/Assets/Archive/bullet_hole_01_Mat.bullet_hole_01_Mat" "7.000000,7.000000,7.000000" OtherComp "None" (Math|Transform|InverseTransformLocation _returnvalue_2 _impactpoint) (Math|Transform|InverseTransformRotation _returnvalue_2 (Transformation|GetWorldRotation MyComp)) "KeepRelativeOffset" 1e+01))
          (Utilities|IsValid _returnvalue_3
            (:Is%20Valid
              (Rendering|Components|Decal|SetFadeScreenSize _returnvalue_3 0.0001))
            (:Is%20Not%20Valid
              _))))
      (Actor|DestroyActor))
    (:NewEnumerator1
      (Effects|SpawnEmitteratLocation "/Game/Assets/FX/P_RocketLauncher_Explosion_01.P_RocketLauncher_Explosion_01" HitLocation)
      (Audio|PlaySoundatLocation "/Game/Assets/Sound/RocketLauncher/RocketLauncher_Explosion_Cue.RocketLauncher_Explosion_Cue" HitLocation "0, 0, 0" 1.0 1.0 0.0 0 0 0)
      (Game|Damage|ApplyRadialDamage (Variables|Default|GetDamage) HitLocation 0.0 0 0 0 0 false "ECC_Visibility")
      (Actor|DestroyActor))))

(fn ConstructionScript)