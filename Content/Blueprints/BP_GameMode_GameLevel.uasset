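; Game mode for the game level, running a countdown that shows a game-over screen at zero and a win screen once no AI enemies remain.
; A looping timer triggers every BP_EnemySpawn until MaxEnemiesOnMap is reached, then stops permanently.
; A second timer polls the AI count for the win, and both end screens pause the game.
; UpdateObjectivesProgress flags weapon-based kill objectives and refreshes the objectives widget.
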(event Custom|Spawn%20Enemy
  ;[1 1 1] Spawn enemies
  (bind _outactors (Actor|GetAllActorsOfClass "/Game/Blueprints/AI/BP_EnemySpawn.BP_EnemySpawn_C"))
  (bind _array_element (Utilities|Array|ForEachLoopwithBreak _outactors :!label _label)
    (:LoopBody
      (bind _outactors_2 (Actor|GetAllActorsOfClass "/Game/Blueprints/AI/BP_Ai_Master.BP_Ai_Master_C"))
      (if (< (Utilities|Array|Length _outactors_2) (Variables|Default|GetMaxEnemiesOnMap))
        (Default|SpawnEnemy _array_element)
        (else
          (Utilities|Time|ClearandInvalidateTimerbyHandle (Variables|Default|GetSpawnTimer))
          (goto _label Break))))))

(event Custom|UpdateObjectivesProgress
  (params (ObjectiveName :type Name))
  (switch name ObjectiveName
    (:Headshot
      (Variables|Default|SetHeadshotObectiveCompleted? true)
      (Variables|Default|SetObjectiveIndex 0))
    (:Shotgun
      (Variables|Default|SetShotgunKillsCompleted? true)
      (Variables|Default|SetObjectiveIndex 1))
    (:Rifle
      (Variables|Default|SetRifleKillsCompleted? true)
      (Variables|Default|SetObjectiveIndex 2))
    (:Pistol
      (Variables|Default|SetPistolKillsCompleted? true)
      (Variables|Default|SetObjectiveIndex 3))
    (:HandGrenade
      (Variables|Default|SetGrenadeKillsCompleted? true)
      (Variables|Default|SetObjectiveIndex 4)))
  (bind _foundwidgets (Widget|GetAllWidgetsOfClass "/Game/UMG/GameLevel/WD_Objectives.WD_Objectives_C" true))
  (for _array_element (Variables|Default|GetPlayerObjectives)
    (UserInterface|Viewport|AddtoViewport (Utilities|Array|Get(acopy) _foundwidgets) 0)
    (Default|UpdateObjectives (Utilities|Array|Get(acopy) _foundwidgets) (Utilities|Select :Index (Variables|Default|GetObjectiveIndex) :Option%200 _array_element :Option%201 _array_element :Option%202 _array_element :Option%203 _array_element :Option%204 _array_element))))

(event Custom|CheckAiNumber
  (bind _returnvalue (Game|GetPlayerController 0))
  ;[1 1 1] Spawn enemies
  (bind _outactors (Actor|GetAllActorsOfClass "/Game/Blueprints/AI/BP_Ai_Master.BP_Ai_Master_C"))
  (if (== (Utilities|Array|Length _outactors) 0)
    (Utilities|FlowControl|DoOnce false
      (:Completed
        (bind _returnvalue_2 (UserInterface|CreateWidget "/Game/UMG/GameLevel/WD_WinScreen.WD_WinScreen_C"))
        (UserInterface|Viewport|AddtoViewport _returnvalue_2 0)
        (Input|SetInputModeUIOnly _returnvalue _returnvalue_2 "LockInFullscreen")
        (Variables|/Script/Engine.PlayerController|SetbShowMouseCursor _returnvalue true)
        (Game|SetGamePaused true)))))

(event EventTick
  (params (DeltaSeconds :type Float%20%28single-precision%29))
  ;[1 1 1] Timer
  (Utilities|FlowControl|Delay 1.0)
  (CallFunction|ExecuteTimer))

(event EventBeginPlay
  ;[1 1 1] Spawn enemies
  (bind _returnvalue (Utilities|Time|SetTimerbyEvent (delegate Custom|Spawn%20Enemy) 1.0 true))
  (Variables|Default|SetSpawnTimer _returnvalue)
  (Utilities|Time|SetTimerbyEvent (delegate Custom|CheckAiNumber) 4.0 true))

(fn ConstructionScript)

(fn ExecuteTimer
  (bind _returnvalue (Game|GetPlayerController 0))
  (if (== (Variables|Default|GetSeconds) 0)
    (if (== (Variables|Default|GetMinutes) 0)
      (bind _returnvalue_2 (UserInterface|CreateWidget "/Game/UMG/GameLevel/WD_GameOver.WD_GameOver_C"))
      (UserInterface|Viewport|AddtoViewport _returnvalue_2 0)
      (Input|SetInputModeUIOnly _returnvalue _returnvalue_2 "LockInFullscreen")
      (Variables|/Script/Engine.PlayerController|SetbShowMouseCursor _returnvalue true)
      (Game|SetGamePaused true)
      (else
        (Variables|Default|SetSeconds 59)
        (Math|Integer|DecrementInt (Variables|Default|GetMinutes))))
    (else
      (Math|Integer|DecrementInt (Variables|Default|GetSeconds)))))